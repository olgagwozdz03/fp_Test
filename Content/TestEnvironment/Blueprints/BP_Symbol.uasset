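; BP_Symbol is a test-environment symbol actor that measures how long the player looks at it.
; Each Tick it dots the camera's forward vector with the direction to the actor; above a tight threshold it sets CzyWykryto (detected), accumulates CzasPatrzenia (gaze time) and prints it.
; PokazSymbol and UkryjSymbol show and hide the TextRender and set Aktywny (active), which the gaze check ignores.
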(event `self.ReceiveTick`
  (params (DeltaSeconds :type "Float (single-precision)"))
  (bind _returnvalue (`GameplayStatics.GetPlayerCameraManager` 0))
  (if true
    (if (> (`KismetMathLibrary.Dot_VectorVector` (`KismetMathLibrary.GetForwardVector` (`PlayerCameraManager.GetCameraRotation` _returnvalue)) (`KismetMathLibrary.GetForwardVector` (`KismetMathLibrary.FindLookAtRotation` (`PlayerCameraManager.GetCameraLocation` _returnvalue) (`self.K2_GetActorLocation`)))) 0.99)
      (set `self.czyWykryto` true)
      (bind _output_get (set `self.czasPatrzenia` (+ (`self.czasPatrzenia`) (`GameplayStatics.GetWorldDeltaSeconds`))))
      (`KismetSystemLibrary.PrintString` (`KismetStringLibrary.Conv_DoubleToString` _output_get)))))

(event `PokazSymbol`
  (set `self.aktywny` true)
  (`SceneComponent.SetVisibility` (`self.TextRender`) true false))

(event `UkryjSymbol`
  (set `self.aktywny` false)
  (`SceneComponent.SetVisibility` (`self.TextRender`) false false))

(fn `UserConstructionScript`)